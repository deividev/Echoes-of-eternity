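; BP_ButtonSequenceManager tracks an ordered button puzzle that opens doors.
; CheckIndex forwards to ButtonPressed, which advances CurrentIndex when the pressed index matches it; wrong presses only print, without resetting progress.
; At three correct presses, it finds every BP_OpenDoor and calls DoorAnimation.
; Other correct presses print debug status, reporting the puzzle as OK at five.
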(event `self.ReceiveBeginPlay`
  (set `self.CurrentIndex` 0))

(event `ButtonPressed`
  (params (ButtonIndex :type Integer))
  (if (== ButtonIndex (`self.CurrentIndex`))
    (bind _output_get (set `self.CurrentIndex` (+ (`self.CurrentIndex`) 1)))
    (if (== _output_get 3)
      (bind _outactors (`GameplayStatics.GetAllActorsOfClass` "/Game/AssetHere/Bps/BP_OpenDoor.BP_OpenDoor_C"))
      (for _array_element _outactors
        (bind _asbp_open_door (cast `/Game/AssetHere/Bps/BP_OpenDoor` _array_element))
        (`/Game/AssetHere/Bps/BP_OpenDoor.DoorAnimation` _asbp_open_door))
      (elif (== _output_get 5)
        (`KismetSystemLibrary.PrintString` "Puzzle  OK")
        (else
          (`KismetSystemLibrary.PrintString` "Puzzle false"))))
    (else
      (`KismetSystemLibrary.PrintString` "False"))))

(fn `CheckIndex`
  (params (ButtonIndex :type Integer))
  (`self.ButtonPressed` ButtonIndex))

(fn `UserConstructionScript`)