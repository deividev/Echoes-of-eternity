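; Rotating puzzle column that the player turns with E while inside its trigger box, which also shows an interaction widget.
; Each press locks input, plays audio and uses a timeline to rotate the Arrow component 90 degrees in yaw.
; On finish it advances a four-step symbol index, sets IsActivated on the last step, and tells BP_Door to recheck its switches.
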(event `Key|E`
  (params (Key :type "Key Structure"))
  (bind _returnvalue (`GameplayStatics.GetPlayerController` 0))
  (bind _currentrotation (`self.CurrentRotation`))
  (bind _returnvalue_2 (+ (`self.PositionOkSimbol`) 1))
  (:`Pressed`
    (`self.DisableInput` _returnvalue)
    (`|ExecutionSequence`
      (:`then_0`
        (bind _output_get (set `self.TargetRotation` (+ _currentrotation 90.0)))
        (`AddComponent|NODE_AddAudioComponent-1`)
        (bind (_direction _animcolumns) (`Timeline|Timeline` :!label _label)
          (:`Update`
            (`SceneComponent.K2_SetRelativeRotation` (`self.Arrow`) (`KismetMathLibrary.MakeRotator` 0.0 0.0 (`KismetMathLibrary.Lerp` _currentrotation _output_get _animcolumns)) false false))
          (:`Finished`
            (`self.EnableInput` _returnvalue)
            (set `self.CurrentRotation` (`self.TargetRotation`))
            (set `self.PositionTriangleSimbol` (`self.K2_GetActorLocation` (`ChildActorComponent.ChildActor` (`self.BP_SimbolTriangle`))))
            (if (== _returnvalue_2 4)
              (set `self.PositionOkSimbol` 0)
              (else
                (bind _output_get_2 (set `self.PositionOkSimbol` _returnvalue_2))))
            (set `self.IsActivated` (== _output_get_2 3))
            (bind _returnvalue_3 (`GameplayStatics.GetActorOfClass` "/Game/AssetHere/Bps/BP_Door.BP_Door_C"))
            (bind _asbp_door (cast `/Game/AssetHere/Bps/BP_Door` _returnvalue_3))
            (`/Game/AssetHere/Bps/BP_Door.OnSwitchActivated` _asbp_door)
            (`/Game/AssetHere/Bps/BP_Door.Check Switches` _asbp_door))))
      (:`then_1`
        (`AddComponent|NODE_AddAudioComponent-0`)
        (goto _label :!via `PlayFromStart`)))))

(event `self.Box1.OnComponentBeginOverlap`
  (params (OverlappedComponent :type "PrimitiveComponent Object Reference") (OtherActor :type "Actor Object Reference") (OtherComp :type "PrimitiveComponent Object Reference") (OtherBodyIndex :type Integer) (bFromSweep :type Boolean) (SweepResult :type "HitResult Structure (by ref)"))
  (cast `/Game/FirstPerson/Blueprints/BP_FirstPersonCharacter` OtherActor)
  (`self.EnableInput` (`GameplayStatics.GetPlayerController` 0))
  (bind _returnvalue (`|CreateWidget` "/Game/AssetHere/Interface/InterfaceInteraction.InterfaceInteraction_C"))
  (`UserWidget.AddToViewport` _returnvalue 0))

(event `self.Box1.OnComponentEndOverlap`
  (params (OverlappedComponent :type "PrimitiveComponent Object Reference") (OtherActor :type "Actor Object Reference") (OtherComp :type "PrimitiveComponent Object Reference") (OtherBodyIndex :type Integer))
  (cast `/Game/FirstPerson/Blueprints/BP_FirstPersonCharacter` OtherActor)
  (`self.DisableInput` (`GameplayStatics.GetPlayerController` 0))
  (`Widget.RemoveFromParent` (stale `self.Box1.OnComponentBeginOverlap` _returnvalue)))

(fn `UserConstructionScript`)