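; BP_OpenDoor is a puzzle door that opens once both the rotating platform and rotating columns are activated.
; CheckSwitches finds one BP_RotatePlatform and one BP_RotateColumns by class, reads their IsActivated flags and fires DoorAnimation if still closed.
; DoorAnimation plays audio and runs a timeline that only acts as a ticker, nudging the door along negative world X by a fixed step per update, making travel frame-rate dependent.
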(event `self.ReceiveBeginPlay`
  (set `self.IsOpen` false))

(event `self.ReceiveTick`
  (params (DeltaSeconds :type "Float (single-precision)")))

(event `DoorAnimation`
  (bind _door (`self.Door`))
  (bind (_returnvalue_x _returnvalue_y _returnvalue_z) (`KismetMathLibrary.BreakVector` (`SceneComponent.K2_GetComponentLocation` _door)))
  (bind _returnvalue (`AddComponent|NODE_AddAudioComponent-0`))
  (`AudioComponent.Play` _returnvalue 0.0)
  (`Timeline|DoorAnim`
    (:`Update`
      _)
    (:`Finished`
      _))
  (`SceneComponent.K2_SetWorldLocation` _door (`KismetMathLibrary.MakeVector` (+ _returnvalue_x -5.0) _returnvalue_y _returnvalue_z) false false)
  (set `self.IsOpen` true))

(fn `Check Switches`
  (`KismetSystemLibrary.PrintString` "Switch" true true (struct :`R` 1.0 :`B` 0.019485 :`A` 1.0))
  (bind _returnvalue (`GameplayStatics.GetActorOfClass` "/Game/AssetHere/Bps/BP_RotatePlatform.BP_RotatePlatform_C"))
  (bind _returnvalue_2 (`GameplayStatics.GetActorOfClass` "/Game/AssetHere/Bps/BP_RotateColumns.BP_RotateColumns_C"))
  (bind _returnvalue_3 (and (`/Game/AssetHere/Bps/BP_RotateColumns.IsActivated` _returnvalue_2) (`/Game/AssetHere/Bps/BP_RotatePlatform.IsActivated` _returnvalue)))
  (if _returnvalue_3
    (if (not (`self.IsOpen`))
      (`self.DoorAnimation`))
    (else
      (`KismetSystemLibrary.PrintString` (`KismetStringLibrary.Conv_BoolToString` _returnvalue_3) true true (struct :`R` 1.0 :`G` 0.010252 :`B` 0.994338 :`A` 1.0)))))

(fn `UserConstructionScript`)